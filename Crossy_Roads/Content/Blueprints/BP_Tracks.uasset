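; Train track tile for a Crossy Road-style game that scores the chicken's crossing and occasionally sends a train across it.
; A Delay-throttled Tick randomly triggers a train sound and blinking warning light before spawning BP_Train.
; BeginPlay randomly spawns up to three coins through nested rolls.
; Overlap volumes add one point through a DoOnce, destroy arriving trains, and remove the tile when the chicken reaches Mapdestroy.
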(event OnComponentBeginOverlap(TrainDestroy)
  (params (OverlappedComponent :type Primitive%20Component%20Object%20Reference) (OtherActor :type Actor%20Object%20Reference) (OtherComp :type Primitive%20Component%20Object%20Reference) (OtherBodyIndex :type Integer) (bFromSweep :type Boolean) (SweepResult :type Hit%20Result%20Structure%20%28by%20ref%29))
  (bind _asbp_train (Utilities|Casting|CastToBP_Train OtherActor))
  (Actor|DestroyActor _asbp_train))

(event OnComponentBeginOverlap(Mapdestroy)
  (params (OverlappedComponent :type Primitive%20Component%20Object%20Reference) (OtherActor :type Actor%20Object%20Reference) (OtherComp :type Primitive%20Component%20Object%20Reference) (OtherBodyIndex :type Integer) (bFromSweep :type Boolean) (SweepResult :type Hit%20Result%20Structure%20%28by%20ref%29))
  (Utilities|Casting|CastToBP_Chicken OtherActor)
  (Actor|DestroyActor))

(event OnComponentBeginOverlap(Box3)
  (params (OverlappedComponent :type Primitive%20Component%20Object%20Reference) (OtherActor :type Actor%20Object%20Reference) (OtherComp :type Primitive%20Component%20Object%20Reference) (OtherBodyIndex :type Integer) (bFromSweep :type Boolean) (SweepResult :type Hit%20Result%20Structure%20%28by%20ref%29))
  (Utilities|FlowControl|DoOnce false
    (:Completed
      (Utilities|Casting|CastToBP_Chicken OtherActor)
      (bind _ascrossy_gm (Utilities|Casting|CastToCrossy_GM (Game|GetGameMode)))
      (Variables|/Game/GameModes/Crossy_GM.Crossy_GM_C|SetScore _ascrossy_gm (+ 1 (Variables|/Game/GameModes/Crossy_GM.Crossy_GM_C|GetScore _ascrossy_gm))))))

(event EventBeginPlay
  (|CallParentFunction)
  (CallFunction|SpawnCoin))

(event Collision|EventActorBeginOverlap
  (params (OtherActor :type Actor%20Object%20Reference)))

(event EventTick
  (params (DeltaSeconds :type Float%20%28single-precision%29))
  (Utilities|FlowControl|Delay 1.0)
  (switch int (Math|Random|RandomIntegerinRange 0 10)
    (:1
      (Utilities|FlowControl|Delay 1.0)
      (Rendering|ToggleVisibility (Variables|Default|GetPointLight) false)
      (Audio|PlaySoundatLocation "/Game/Audio/C_Train.C_Train" (Transformation|GetWorldLocation (Variables|Default|GetTrainPost)) "0, 0, 0" 1.0 1.0 0.0 0 0 0)
      (Utilities|FlowControl|Delay 1.0)
      (Rendering|ToggleVisibility (Variables|Default|GetPointLight) false)
      (Utilities|FlowControl|Delay 1.0)
      (Rendering|ToggleVisibility (Variables|Default|GetPointLight) false)
      (Utilities|FlowControl|Delay 1.0)
      (Rendering|ToggleVisibility (Variables|Default|GetPointLight) false)
      (Utilities|FlowControl|Delay 1.0)
      (Game|SpawnActorfromClass "/Game/Blueprints/BP_Train.BP_Train_C" (Transformation|GetWorldTransform (Variables|Default|GetTrainSpawn)) "Undefined" 0 0))))

(fn ConstructionScript
  (|CallParentFunction))

(fn SpawnTrains)

(fn SpawnCoin
  (switch int (Math|Random|RandomIntegerinRange 0 5)
    (:0
      (Game|SpawnActorfromClass "/Game/Blueprints/BP_Coin.BP_Coin_C" (Transformation|GetWorldTransform (Variables|Default|GetArrow12)) "Undefined" 0 0)
      (switch int (Math|Random|RandomIntegerinRange 0 5)
        (:0
          (Game|SpawnActorfromClass "/Game/Blueprints/BP_Coin.BP_Coin_C" (Transformation|GetWorldTransform (Variables|Default|GetArrow13)) "Undefined" 0 0)
          (switch int (Math|Random|RandomIntegerinRange 0 5)
            (:0
              (Game|SpawnActorfromClass "/Game/Blueprints/BP_Coin.BP_Coin_C" (Transformation|GetWorldTransform (Variables|Default|GetArrow14)) "Undefined" 0 0))))))))