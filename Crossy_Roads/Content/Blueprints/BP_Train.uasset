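; BP_Train is a train hazard that kills the chicken on contact and sends the game back to the main menu.
; It adds its mesh at BeginPlay and moves along local X on Tick at MaxSpeed.
; Overlapping ChickenTrainDeath with a BP_Chicken spawns an explosion, then destroys the chicken and opens MainMenu after a short delay.
; A BP_Cars spawn at TrainSpawn is left unwired and never runs.
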(event OnComponentBeginOverlap(ChickenTrainDeath)
  (params (OverlappedComponent :type Primitive%20Component%20Object%20Reference) (OtherActor :type Actor%20Object%20Reference) (OtherComp :type Primitive%20Component%20Object%20Reference) (OtherBodyIndex :type Integer) (bFromSweep :type Boolean) (SweepResult :type Hit%20Result%20Structure%20%28by%20ref%29))
  (bind _asbp_chicken (Utilities|Casting|CastToBP_Chicken OtherActor))
  (Effects|SpawnEmitteratLocation "/Game/Particles/Explosion.Explosion" (Transformation|GetActorLocation _asbp_chicken))
  (Utilities|FlowControl|Delay 1.0)
  (Actor|DestroyActor _asbp_chicken)
  (Game|OpenLevel(byName) "MainMenu"))

(event EventBeginPlay
  (bind _returnvalue (AddComponent|AddStaticMeshComponent false))
  (Components|StaticMesh|SetStaticMesh _returnvalue "/Game/Meshes/train.train"))

(event Collision|EventActorBeginOverlap
  (params (OtherActor :type Actor%20Object%20Reference)))

(event EventTick
  (params (DeltaSeconds :type Float%20%28single-precision%29))
  (Transformation|AddActorLocalOffset (Math|Vector|MakeVector (* DeltaSeconds (Variables|Default|GetMaxSpeed)) 0.0 0.0) false false))

(fn ConstructionScript)