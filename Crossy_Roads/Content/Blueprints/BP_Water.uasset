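; Water row for a Crossy Road-style game that holds either lily pads or logs, chosen at random on BeginPlay.
; Lily pads spawn once at random preset points, while log rows use a Delay on Tick to randomly spawn logs, which side triggers destroy.
; A chicken scores once on crossing Box3 and removes the row on reaching Mapdestroy.
; Hitting the water plays an effect, destroys the chicken and opens MainMenu.
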(event OnComponentBeginOverlap(Mapdestroy)
  (params (OverlappedComponent :type Primitive%20Component%20Object%20Reference) (OtherActor :type Actor%20Object%20Reference) (OtherComp :type Primitive%20Component%20Object%20Reference) (OtherBodyIndex :type Integer) (bFromSweep :type Boolean) (SweepResult :type Hit%20Result%20Structure%20%28by%20ref%29))
  (Utilities|Casting|CastToBP_Chicken OtherActor)
  (Actor|DestroyActor))

(event OnComponentBeginOverlap(LogDestroy)
  (params (OverlappedComponent :type Primitive%20Component%20Object%20Reference) (OtherActor :type Actor%20Object%20Reference) (OtherComp :type Primitive%20Component%20Object%20Reference) (OtherBodyIndex :type Integer) (bFromSweep :type Boolean) (SweepResult :type Hit%20Result%20Structure%20%28by%20ref%29))
  (bind _asbp_logs (Utilities|Casting|CastToBP_Logs OtherActor))
  (Actor|DestroyActor _asbp_logs))

(event OnComponentBeginOverlap(LogDestroy2)
  (params (OverlappedComponent :type Primitive%20Component%20Object%20Reference) (OtherActor :type Actor%20Object%20Reference) (OtherComp :type Primitive%20Component%20Object%20Reference) (OtherBodyIndex :type Integer) (bFromSweep :type Boolean) (SweepResult :type Hit%20Result%20Structure%20%28by%20ref%29))
  (bind _asbp_logs (Utilities|Casting|CastToBP_Logs OtherActor))
  (Actor|DestroyActor _asbp_logs))

(event OnComponentBeginOverlap(Box3)
  (params (OverlappedComponent :type Primitive%20Component%20Object%20Reference) (OtherActor :type Actor%20Object%20Reference) (OtherComp :type Primitive%20Component%20Object%20Reference) (OtherBodyIndex :type Integer) (bFromSweep :type Boolean) (SweepResult :type Hit%20Result%20Structure%20%28by%20ref%29))
  (Utilities|FlowControl|DoOnce false
    (:Completed
      (Utilities|Casting|CastToBP_Chicken OtherActor)
      (bind _ascrossy_gm (Utilities|Casting|CastToCrossy_GM (Game|GetGameMode)))
      (Variables|/Game/GameModes/Crossy_GM.Crossy_GM_C|SetScore _ascrossy_gm (+ 1 (Variables|/Game/GameModes/Crossy_GM.Crossy_GM_C|GetScore _ascrossy_gm))))))

(event OnComponentHit(WaterMesh)
  (params (HitComponent :type Primitive%20Component%20Object%20Reference) (OtherActor :type Actor%20Object%20Reference) (OtherComp :type Primitive%20Component%20Object%20Reference) (NormalImpulse :type Vector :default "0, 0, 0") (Hit :type Hit%20Result%20Structure%20%28by%20ref%29))
  (bind _asbp_chicken (Utilities|Casting|CastToBP_Chicken OtherActor))
  (Effects|SpawnEmitteratLocation "/Game/Particles/WaterEx.WaterEx" (Transformation|GetActorLocation _asbp_chicken))
  (Utilities|FlowControl|Delay 1.0)
  (Actor|DestroyActor _asbp_chicken)
  (Game|OpenLevel(byName) "MainMenu"))

(event EventBeginPlay
  (|CallParentFunction)
  (if (Math|Random|RandomBool)
    (Variables|Default|SetLilpads true)
    (CallFunction|SpawnLilpads)))

(event Collision|EventActorBeginOverlap
  (params (OtherActor :type Actor%20Object%20Reference)))

(event EventTick
  (params (DeltaSeconds :type Float%20%28single-precision%29))
  (Utilities|FlowControl|Delay 1.0)
  (if (not (Variables|Default|GetLilpads))
    (CallFunction|SpawnLogs)))

(fn ConstructionScript
  (|CallParentFunction))

(fn SpawnLilpads
  (for _index (range 0 3)
    (switch int (Math|Random|RandomIntegerinRange 0 8)
      (:0
        (Game|SpawnActorfromClass "/Game/Blueprints/BP_Lilpad.BP_Lilpad_C" (Transformation|GetWorldTransform (Variables|Default|GetLilPad1)) "Undefined" 0 0))
      (:1
        (Game|SpawnActorfromClass "/Game/Blueprints/BP_Lilpad.BP_Lilpad_C" (Transformation|GetWorldTransform (Variables|Default|GetLilpad5)) "Undefined" 0 0))
      (:2
        (Game|SpawnActorfromClass "/Game/Blueprints/BP_Lilpad.BP_Lilpad_C" (Transformation|GetWorldTransform (Variables|Default|GetLilpad2)) "Undefined" 0 0))
      (:3
        (Game|SpawnActorfromClass "/Game/Blueprints/BP_Lilpad.BP_Lilpad_C" (Transformation|GetWorldTransform (Variables|Default|GetLilpad3)) "Undefined" 0 0))
      (:4
        (Game|SpawnActorfromClass "/Game/Blueprints/BP_Lilpad.BP_Lilpad_C" (Transformation|GetWorldTransform (Variables|Default|GetLilpad4)) "Undefined" 0 0))
      (:5
        (Game|SpawnActorfromClass "/Game/Blueprints/BP_Lilpad.BP_Lilpad_C" (Transformation|GetWorldTransform (Variables|Default|GetLilpad8)) "Undefined" 0 0))
      (:6
        (Game|SpawnActorfromClass "/Game/Blueprints/BP_Lilpad.BP_Lilpad_C" (Transformation|GetWorldTransform (Variables|Default|GetLilpad6)) "Undefined" 0 0))
      (:7
        (Game|SpawnActorfromClass "/Game/Blueprints/BP_Lilpad.BP_Lilpad_C" (Transformation|GetWorldTransform (Variables|Default|GetLilpad7)) "Undefined" 0 0))
      (:8
        (Game|SpawnActorfromClass "/Game/Blueprints/BP_Lilpad.BP_Lilpad_C" (Transformation|GetWorldTransform (Variables|Default|GetLilpad9)) "Undefined" 0 0)))))

(fn SpawnLogs
  (switch int (Math|Random|RandomIntegerinRange 0 2)
    (:1
      (Game|SpawnActorfromClass "/Game/Blueprints/BP_Logs.BP_Logs_C" (Transformation|GetWorldTransform (Variables|Default|GetLogSpawn)) "Undefined" 0 0))))