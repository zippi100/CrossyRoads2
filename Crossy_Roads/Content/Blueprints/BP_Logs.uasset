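; BP_Logs is a moving log actor that appears in one of three mesh variants.
; BeginPlay picks SLog, MLog or LLog at random and adds it as a new static mesh component.
; Tick moves the actor along its local X axis at MaxSpeed, scaled by delta time.
; An unconnected node to spawn another BP_Logs at LogSpawn never runs.
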(event EventBeginPlay
  (switch int (Math|Random|RandomIntegerinRange 0 2)
    (:0
      (bind _returnvalue (AddComponent|AddStaticMeshComponent false))
      (Components|StaticMesh|SetStaticMesh _returnvalue "/Game/Meshes/sLog.sLog"))
    (:1
      (bind _returnvalue_2 (AddComponent|AddStaticMeshComponent false))
      (Components|StaticMesh|SetStaticMesh _returnvalue_2 "/Game/Meshes/mLog.mLog"))
    (:2
      (bind _returnvalue_3 (AddComponent|AddStaticMeshComponent false))
      (Components|StaticMesh|SetStaticMesh _returnvalue_3 "/Game/Meshes/lLog.lLog"))))

(event Collision|EventActorBeginOverlap
  (params (OtherActor :type Actor%20Object%20Reference)))

(event EventTick
  (params (DeltaSeconds :type Float%20%28single-precision%29))
  (Transformation|AddActorLocalOffset (Math|Vector|MakeVector (* DeltaSeconds (Variables|Default|GetMaxSpeed)) 0.0 0.0) false false))

(fn ConstructionScript)