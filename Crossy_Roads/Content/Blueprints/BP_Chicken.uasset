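; BP_Chicken is the player character of a Crossy Road-style game, hopping in four directions.
; Each move input plays a timeline that, every update, calls Jump, applies a fixed local offset and turns the mesh, so distance depends on update count.
; BeginPlay shows the Score widget and creates or updates the high-score save from Crossy_GM's score, only at that moment.
; Tick applies pending movement input; movement-disabling nodes are unconnected.
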(event EventBeginPlay
  (bind _returnvalue (UserInterface|CreateWidget "/Game/UI/Score.Score_C"))
  (UserInterface|Viewport|AddtoViewport _returnvalue 0)
  (bind _ascrossy_gm (Utilities|Casting|CastToCrossy_GM (Game|GetGameMode)))
  (bind _returnvalue_2 (SaveGame|DoesSaveGameExist "HighSocreData"))
  (if _returnvalue_2
    (bind _returnvalue_3 (SaveGame|LoadGamefromSlot "HighSocreData"))
    (bind _output_get (Variables|Default|SetSaveSubClass _returnvalue_3))
    (bind _asbp_savegame (Utilities|Casting|CastToBP_Savegame _output_get))
    (if (> (Variables|/Game/GameModes/Crossy_GM.Crossy_GM_C|GetScore _ascrossy_gm) (Variables|/Game/Blueprints/BP_Savegame.BP_Savegame_C|GetHigh_Score _asbp_savegame))
      (Variables|/Game/Blueprints/BP_Savegame.BP_Savegame_C|SetHigh_Score _asbp_savegame (Variables|/Game/GameModes/Crossy_GM.Crossy_GM_C|GetScore _ascrossy_gm))
      (SaveGame|SaveGametoSlot (Variables|Default|GetSaveSubClass) "HighSocreData"))
    (else
      (bind _returnvalue_4 (SaveGame|CreateSaveGameObject))
      (bind _output_get_2 (Variables|Default|SetSaveSubClass _returnvalue_4))
      (bind _asbp_savegame_2 (Utilities|Casting|CastToBP_Savegame _output_get_2))
      (Variables|/Game/Blueprints/BP_Savegame.BP_Savegame_C|SetHigh_Score _asbp_savegame_2 (Variables|/Game/GameModes/Crossy_GM.Crossy_GM_C|GetScore _ascrossy_gm))
      (SaveGame|SaveGametoSlot (Variables|Default|GetSaveSubClass) "HighSocreData"))))

(event EventTick
  (params (DeltaSeconds :type Float%20%28single-precision%29))
  (bind _returnvalue (Class|Pawn|ConsumeMovementInputVector))
  (Transformation|AddActorLocalOffset _returnvalue false false))

(event Input|ActionEvents|InputActionMoveRight
  (params (Key :type Key%20Structure))
  (:Pressed
    (Timeline|Timeline_0 PlayFromStart
      (:Update
        (Character|Jump)
        (Transformation|AddActorLocalOffset "0,15.000000, 0" false false)
        (Transformation|SetRelativeRotation (Variables|Default|GetChickenMesh) "0,360.000000, 0" false false)))))

(event Input|ActionEvents|InputActionMoveForward
  (params (Key :type Key%20Structure))
  (:Pressed
    (Timeline|Timeline_2 PlayFromStart
      (:Update
        (Character|Jump)
        (Transformation|AddActorLocalOffset "15.000000, 0, 0" false false)
        (Transformation|SetRelativeRotation (Variables|Default|GetChickenMesh) "0,270.000000, 0" false false)))))

(event Input|ActionEvents|InputActionMoveBack
  (params (Key :type Key%20Structure))
  (:Pressed
    (Timeline|Timeline_3 PlayFromStart
      (:Update
        (Character|Jump)
        (Transformation|AddActorLocalOffset "-15.000000, 0, 0" false false)
        (Transformation|SetRelativeRotation (Variables|Default|GetChickenMesh) "0,90.000000, 0" false false)))))

(event Input|ActionEvents|InputActionMoveLeft
  (params (Key :type Key%20Structure))
  (:Pressed
    (Timeline|Timeline_1 PlayFromStart
      (:Update
        (Character|Jump)
        (Transformation|AddActorLocalOffset "0.000000,-15.000000, 0" false false)
        (Transformation|SetRelativeRotation (Variables|Default|GetChickenMesh) "0,180.000000, 0" false false)))))

(fn ConstructionScript)