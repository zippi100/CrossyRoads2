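; BP_Water2 is a two-lane water hazard for a Crossy Road-style game, where hitting the water destroys BP_Chicken and opens MainMenu.
; With Lilpads set, both lanes spawn logs; otherwise BeginPlay randomly fills one lane with lilypads and the other spawns logs.
; Tick uses a one-second Delay as a timer for random log spawns.
; Two one-shot trigger boxes increment the Crossy_GM score, though any actor's overlap consumes them.
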(event OnComponentBeginOverlap(Box4)
  (params (OverlappedComponent :type Primitive%20Component%20Object%20Reference) (OtherActor :type Actor%20Object%20Reference) (OtherComp :type Primitive%20Component%20Object%20Reference) (OtherBodyIndex :type Integer) (bFromSweep :type Boolean) (SweepResult :type Hit%20Result%20Structure%20%28by%20ref%29))
  (Utilities|FlowControl|DoOnce false
    (:Completed
      (Utilities|Casting|CastToBP_Chicken OtherActor)
      (bind _ascrossy_gm (Utilities|Casting|CastToCrossy_GM (Game|GetGameMode)))
      (Variables|/Game/GameModes/Crossy_GM.Crossy_GM_C|SetScore _ascrossy_gm (+ 1 (Variables|/Game/GameModes/Crossy_GM.Crossy_GM_C|GetScore _ascrossy_gm))))))

(event OnComponentBeginOverlap(Box5)
  (params (OverlappedComponent :type Primitive%20Component%20Object%20Reference) (OtherActor :type Actor%20Object%20Reference) (OtherComp :type Primitive%20Component%20Object%20Reference) (OtherBodyIndex :type Integer) (bFromSweep :type Boolean) (SweepResult :type Hit%20Result%20Structure%20%28by%20ref%29))
  (Utilities|FlowControl|DoOnce false
    (:Completed
      (Utilities|Casting|CastToBP_Chicken OtherActor)
      (bind _ascrossy_gm (Utilities|Casting|CastToCrossy_GM (Game|GetGameMode)))
      (Variables|/Game/GameModes/Crossy_GM.Crossy_GM_C|SetScore _ascrossy_gm (+ 1 (Variables|/Game/GameModes/Crossy_GM.Crossy_GM_C|GetScore _ascrossy_gm))))))

(event OnComponentHit(StaticMesh_0)
  (params (HitComponent :type Primitive%20Component%20Object%20Reference) (OtherActor :type Actor%20Object%20Reference) (OtherComp :type Primitive%20Component%20Object%20Reference) (NormalImpulse :type Vector :default "0, 0, 0") (Hit :type Hit%20Result%20Structure%20%28by%20ref%29))
  (bind _asbp_chicken (Utilities|Casting|CastToBP_Chicken OtherActor))
  (Effects|SpawnEmitteratLocation "/Game/Particles/WaterEx.WaterEx" (Transformation|GetActorLocation _asbp_chicken))
  (Utilities|FlowControl|Delay 1.0)
  (Actor|DestroyActor _asbp_chicken)
  (Game|OpenLevel(byName) "MainMenu"))

(event OnComponentHit(StaticMesh1)
  (params (HitComponent :type Primitive%20Component%20Object%20Reference) (OtherActor :type Actor%20Object%20Reference) (OtherComp :type Primitive%20Component%20Object%20Reference) (NormalImpulse :type Vector :default "0, 0, 0") (Hit :type Hit%20Result%20Structure%20%28by%20ref%29))
  (bind _asbp_chicken (Utilities|Casting|CastToBP_Chicken OtherActor))
  (Effects|SpawnEmitteratLocation "/Game/Particles/WaterEx.WaterEx" (Transformation|GetActorLocation _asbp_chicken))
  (Utilities|FlowControl|Delay 1.0)
  (Actor|DestroyActor _asbp_chicken)
  (Game|OpenLevel(byName) "MainMenu"))

(event EventBeginPlay
  (|CallParentFunction)
  (if (not (Variables|Default|GetLilpads))
    (switch int (Math|Random|RandomIntegerinRange 0 1)
      (:0
        (Variables|Default|Setlil2 false)
        (CallFunction|SpawnLil2))
      (:1
        (Variables|Default|Setlil2 true)
        (CallFunction|SpawnLil1)))))

(event Collision|EventActorBeginOverlap
  (params (OtherActor :type Actor%20Object%20Reference))
  (|CallParentFunction OtherActor) ; This node is disabled and will not be called.\nDrag off pins to build functionality.
)

(event EventTick
  (params (DeltaSeconds :type Float%20%28single-precision%29))
  (|CallParentFunction DeltaSeconds)
  (if (Variables|Default|GetLilpads)
    (Utilities|FlowControl|Delay 1.0)
    (CallFunction|SpawnLogs1)
    (CallFunction|SpawnLogs2)
    (elif (Variables|Default|Getlil2)
      (Utilities|FlowControl|Delay 1.0)
      (CallFunction|SpawnLogs4)
      (else
        (Utilities|FlowControl|Delay 1.0)
        (CallFunction|SpawnLogs3)))))

(fn ConstructionScript
  (|CallParentFunction))

(fn SpawnLogs1
  (switch int (Math|Random|RandomIntegerinRange 0 3)
    (:1
      (Game|SpawnActorfromClass "/Game/Blueprints/BP_Logs.BP_Logs_C" (Transformation|GetWorldTransform (Variables|Default|GetArrow22)) "Undefined" 0 0))))

(fn SpawnLogs2
  (switch int (Math|Random|RandomIntegerinRange 0 3)
    (:1
      (Game|SpawnActorfromClass "/Game/Blueprints/BP_Logs.BP_Logs_C" (Transformation|GetWorldTransform (Variables|Default|GetArrow9_0)) "Undefined" 0 0))))

(fn SpawnLil1
  (for _index (range 0 3)
    (switch int (Math|Random|RandomIntegerinRange 0 7)
      (:0
        (Game|SpawnActorfromClass "/Game/Blueprints/BP_Lilpad.BP_Lilpad_C" (Transformation|GetWorldTransform (Variables|Default|GetArrow3_0)) "Undefined" 0 0))
      (:1
        (Game|SpawnActorfromClass "/Game/Blueprints/BP_Lilpad.BP_Lilpad_C" (Transformation|GetWorldTransform (Variables|Default|GetArrow8_0)) "Undefined" 0 0))
      (:2
        (Game|SpawnActorfromClass "/Game/Blueprints/BP_Lilpad.BP_Lilpad_C" (Transformation|GetWorldTransform (Variables|Default|GetArrow1_0)) "Undefined" 0 0))
      (:3
        (Game|SpawnActorfromClass "/Game/Blueprints/BP_Lilpad.BP_Lilpad_C" (Transformation|GetWorldTransform (Variables|Default|GetArrow6_0)) "Undefined" 0 0))
      (:4
        (Game|SpawnActorfromClass "/Game/Blueprints/BP_Lilpad.BP_Lilpad_C" (Transformation|GetWorldTransform (Variables|Default|GetArrow2_0)) "Undefined" 0 0))
      (:5
        (Game|SpawnActorfromClass "/Game/Blueprints/BP_Lilpad.BP_Lilpad_C" (Transformation|GetWorldTransform (Variables|Default|GetArrow5_0)) "Undefined" 0 0))
      (:6
        (Game|SpawnActorfromClass "/Game/Blueprints/BP_Lilpad.BP_Lilpad_C" (Transformation|GetWorldTransform (Variables|Default|GetArrow7_0)) "Undefined" 0 0))
      (:7
        (Game|SpawnActorfromClass "/Game/Blueprints/BP_Lilpad.BP_Lilpad_C" (Transformation|GetWorldTransform (Variables|Default|GetArrow4_0)) "Undefined" 0 0)))))

(fn SpawnLil2
  (for _index (range 0 3)
    (switch int (Math|Random|RandomIntegerinRange 0 7)
      (:0
        (Game|SpawnActorfromClass "/Game/Blueprints/BP_Lilpad.BP_Lilpad_C" (Transformation|GetWorldTransform (Variables|Default|GetArrow13)) "Undefined" 0 0))
      (:1
        (Game|SpawnActorfromClass "/Game/Blueprints/BP_Lilpad.BP_Lilpad_C" (Transformation|GetWorldTransform (Variables|Default|GetArrow18)) "Undefined" 0 0))
      (:2
        (Game|SpawnActorfromClass "/Game/Blueprints/BP_Lilpad.BP_Lilpad_C" (Transformation|GetWorldTransform (Variables|Default|GetArrow11_0)) "Undefined" 0 0))
      (:3
        (Game|SpawnActorfromClass "/Game/Blueprints/BP_Lilpad.BP_Lilpad_C" (Transformation|GetWorldTransform (Variables|Default|GetArrow16)) "Undefined" 0 0))
      (:4
        (Game|SpawnActorfromClass "/Game/Blueprints/BP_Lilpad.BP_Lilpad_C" (Transformation|GetWorldTransform (Variables|Default|GetArrow12)) "Undefined" 0 0))
      (:5
        (Game|SpawnActorfromClass "/Game/Blueprints/BP_Lilpad.BP_Lilpad_C" (Transformation|GetWorldTransform (Variables|Default|GetArrow14)) "Undefined" 0 0))
      (:6
        (Game|SpawnActorfromClass "/Game/Blueprints/BP_Lilpad.BP_Lilpad_C" (Transformation|GetWorldTransform (Variables|Default|GetArrow17)) "Undefined" 0 0))
      (:7
        (Game|SpawnActorfromClass "/Game/Blueprints/BP_Lilpad.BP_Lilpad_C" (Transformation|GetWorldTransform (Variables|Default|GetArrow15)) "Undefined" 0 0)))))

(fn SpawnLogs3
  (switch int (Math|Random|RandomIntegerinRange 0 3)
    (:1
      (Game|SpawnActorfromClass "/Game/Blueprints/BP_Logs.BP_Logs_C" (Transformation|GetWorldTransform (Variables|Default|GetArrow21)) "Undefined" 0 0))))

(fn SpawnLogs4
  (switch int (Math|Random|RandomIntegerinRange 0 3)
    (:1
      (Game|SpawnActorfromClass "/Game/Blueprints/BP_Logs.BP_Logs_C" (Transformation|GetWorldTransform (Variables|Default|GetArrow22)) "Undefined" 0 0))))