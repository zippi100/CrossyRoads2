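; Road tile for a Crossy Road-style game that spawns traffic and coins, and awards score to the chicken.
; A Delay on Tick paces random car or truck spawns at either of two points per type, with end triggers destroying the vehicles.
; BeginPlay rolls a nested chain of coin spawns, each requiring the previous.
; Two one-shot boxes increment Crossy_GM's Score, and Mapdestroy removes the tile when the chicken overlaps it.
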(event OnComponentBeginOverlap(Box3)
  (params (OverlappedComponent :type Primitive%20Component%20Object%20Reference) (OtherActor :type Actor%20Object%20Reference) (OtherComp :type Primitive%20Component%20Object%20Reference) (OtherBodyIndex :type Integer) (bFromSweep :type Boolean) (SweepResult :type Hit%20Result%20Structure%20%28by%20ref%29))
  (Utilities|FlowControl|DoOnce false
    (:Completed
      (Utilities|Casting|CastToBP_Chicken OtherActor)
      (bind _ascrossy_gm (Utilities|Casting|CastToCrossy_GM (Game|GetGameMode)))
      (Variables|/Game/GameModes/Crossy_GM.Crossy_GM_C|SetScore _ascrossy_gm (+ 1 (Variables|/Game/GameModes/Crossy_GM.Crossy_GM_C|GetScore _ascrossy_gm))))))

(event OnComponentBeginOverlap(Box4)
  (params (OverlappedComponent :type Primitive%20Component%20Object%20Reference) (OtherActor :type Actor%20Object%20Reference) (OtherComp :type Primitive%20Component%20Object%20Reference) (OtherBodyIndex :type Integer) (bFromSweep :type Boolean) (SweepResult :type Hit%20Result%20Structure%20%28by%20ref%29))
  (Utilities|FlowControl|DoOnce false
    (:Completed
      (Utilities|Casting|CastToBP_Chicken OtherActor)
      (bind _ascrossy_gm (Utilities|Casting|CastToCrossy_GM (Game|GetGameMode)))
      (Variables|/Game/GameModes/Crossy_GM.Crossy_GM_C|SetScore _ascrossy_gm (+ 1 (Variables|/Game/GameModes/Crossy_GM.Crossy_GM_C|GetScore _ascrossy_gm))))))

(event OnComponentBeginOverlap(CarDestoy1)
  (params (OverlappedComponent :type Primitive%20Component%20Object%20Reference) (OtherActor :type Actor%20Object%20Reference) (OtherComp :type Primitive%20Component%20Object%20Reference) (OtherBodyIndex :type Integer) (bFromSweep :type Boolean) (SweepResult :type Hit%20Result%20Structure%20%28by%20ref%29))
  (bind _asbp_cars (Utilities|Casting|CastToBP_Cars OtherActor))
  (Actor|DestroyActor _asbp_cars))

(event OnComponentBeginOverlap(TruckDesroy1)
  (params (OverlappedComponent :type Primitive%20Component%20Object%20Reference) (OtherActor :type Actor%20Object%20Reference) (OtherComp :type Primitive%20Component%20Object%20Reference) (OtherBodyIndex :type Integer) (bFromSweep :type Boolean) (SweepResult :type Hit%20Result%20Structure%20%28by%20ref%29))
  (bind _asbp_truck (Utilities|Casting|CastToBP_Truck OtherActor))
  (Actor|DestroyActor _asbp_truck))

(event OnComponentBeginOverlap(CarDestroy2)
  (params (OverlappedComponent :type Primitive%20Component%20Object%20Reference) (OtherActor :type Actor%20Object%20Reference) (OtherComp :type Primitive%20Component%20Object%20Reference) (OtherBodyIndex :type Integer) (bFromSweep :type Boolean) (SweepResult :type Hit%20Result%20Structure%20%28by%20ref%29))
  (bind _asbp_cars (Utilities|Casting|CastToBP_Cars OtherActor))
  (Actor|DestroyActor _asbp_cars))

(event OnComponentBeginOverlap(TruckDestory2)
  (params (OverlappedComponent :type Primitive%20Component%20Object%20Reference) (OtherActor :type Actor%20Object%20Reference) (OtherComp :type Primitive%20Component%20Object%20Reference) (OtherBodyIndex :type Integer) (bFromSweep :type Boolean) (SweepResult :type Hit%20Result%20Structure%20%28by%20ref%29))
  (bind _asbp_truck (Utilities|Casting|CastToBP_Truck OtherActor))
  (Actor|DestroyActor _asbp_truck))

(event OnComponentBeginOverlap(Mapdestroy)
  (params (OverlappedComponent :type Primitive%20Component%20Object%20Reference) (OtherActor :type Actor%20Object%20Reference) (OtherComp :type Primitive%20Component%20Object%20Reference) (OtherBodyIndex :type Integer) (bFromSweep :type Boolean) (SweepResult :type Hit%20Result%20Structure%20%28by%20ref%29))
  (Utilities|Casting|CastToBP_Chicken OtherActor)
  (Actor|DestroyActor))

(event EventBeginPlay
  (|CallParentFunction)
  (CallFunction|SpawnCoin))

(event Collision|EventActorBeginOverlap
  (params (OtherActor :type Actor%20Object%20Reference)))

(event EventTick
  (params (DeltaSeconds :type Float%20%28single-precision%29))
  (Utilities|FlowControl|Delay 1.2)
  (if (Math|Random|RandomBool)
    (CallFunction|CarSpawns)
    (else
      (CallFunction|TruckSapwn))))

(fn ConstructionScript
  (|CallParentFunction))

(fn CarSpawns
  (if (Math|Random|RandomBool)
    (switch int (Math|Random|RandomIntegerinRange 0 1)
      (:1
        (Game|SpawnActorfromClass "/Game/Blueprints/BP_Cars.BP_Cars_C" (Transformation|GetWorldTransform (Variables|Default|GetCarSpawn1)) "Undefined" 0 0)))
    (else
      (switch int (Math|Random|RandomIntegerinRange 0 1)
        (:1
          (Game|SpawnActorfromClass "/Game/Blueprints/BP_Cars.BP_Cars_C" (Transformation|GetWorldTransform (Variables|Default|GetCarSpawn2)) "Undefined" 0 0))))))

(fn TruckSapwn
  (if (Math|Random|RandomBool)
    (switch int (Math|Random|RandomIntegerinRange 0 1)
      (:1
        (Game|SpawnActorfromClass "/Game/Blueprints/BP_Truck.BP_Truck_C" (Transformation|GetWorldTransform (Variables|Default|GetTruckSpawn1)) "Undefined" 0 0)))
    (else
      (switch int (Math|Random|RandomIntegerinRange 0 1)
        (:1
          (Game|SpawnActorfromClass "/Game/Blueprints/BP_Truck.BP_Truck_C" (Transformation|GetWorldTransform (Variables|Default|GetTruckSpawn2)) "Undefined" 0 0))))))

(fn SpawnCoin
  (switch int (Math|Random|RandomIntegerinRange 0 5)
    (:0
      (Game|SpawnActorfromClass "/Game/Blueprints/BP_Coin.BP_Coin_C" (Transformation|GetWorldTransform (Variables|Default|GetArrow12)) "Undefined" 0 0)
      (switch int (Math|Random|RandomIntegerinRange 0 5)
        (:0
          (Game|SpawnActorfromClass "/Game/Blueprints/BP_Coin.BP_Coin_C" (Transformation|GetWorldTransform (Variables|Default|GetArrow13)) "Undefined" 0 0)
          (switch int (Math|Random|RandomIntegerinRange 0 5)
            (:0
              (Game|SpawnActorfromClass "/Game/Blueprints/BP_Coin.BP_Coin_C" (Transformation|GetWorldTransform (Variables|Default|GetArrow14)) "Undefined" 0 0)
              (switch int (Math|Random|RandomIntegerinRange 0 5)
                (:0
                  (Game|SpawnActorfromClass "/Game/Blueprints/BP_Coin.BP_Coin_C" (Transformation|GetWorldTransform (Variables|Default|GetArrow15)) "Undefined" 0 0)
                  (switch int (Math|Random|RandomIntegerinRange 0 5)
                    (:0
                      (Game|SpawnActorfromClass "/Game/Blueprints/BP_Coin.BP_Coin_C" (Transformation|GetWorldTransform (Variables|Default|GetArrow16)) "Undefined" 0 0)
                      (switch int (Math|Random|RandomIntegerinRange 0 5)
                        (:0
                          (Game|SpawnActorfromClass "/Game/Blueprints/BP_Coin.BP_Coin_C" (Transformation|GetWorldTransform (Variables|Default|GetArrow17)) "Undefined" 0 0))))))))))))))