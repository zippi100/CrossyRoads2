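; Road segment for a Crossy Road-style game that spawns traffic and coins for the chicken to cross.
; A Delay on Tick paces random car or truck spawns at arrow points, while BeginPlay rolls nested chances for up to three coins.
; Overlap volumes destroy vehicles, or the segment itself when the chicken reaches MapDestroy.
; The mesh's first hit passes a DoOnce, adding a point to Crossy_GM's score if it is the chicken.
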(event OnComponentBeginOverlap(CarDestroy)
  (params (OverlappedComponent :type Primitive%20Component%20Object%20Reference) (OtherActor :type Actor%20Object%20Reference) (OtherComp :type Primitive%20Component%20Object%20Reference) (OtherBodyIndex :type Integer) (bFromSweep :type Boolean) (SweepResult :type Hit%20Result%20Structure%20%28by%20ref%29))
  (bind _asbp_cars (Utilities|Casting|CastToBP_Cars OtherActor))
  (Actor|DestroyActor _asbp_cars))

(event OnComponentBeginOverlap(TruckDestroy)
  (params (OverlappedComponent :type Primitive%20Component%20Object%20Reference) (OtherActor :type Actor%20Object%20Reference) (OtherComp :type Primitive%20Component%20Object%20Reference) (OtherBodyIndex :type Integer) (bFromSweep :type Boolean) (SweepResult :type Hit%20Result%20Structure%20%28by%20ref%29))
  (bind _asbp_truck (Utilities|Casting|CastToBP_Truck OtherActor))
  (Actor|DestroyActor _asbp_truck))

(event OnComponentBeginOverlap(MapDestroy)
  (params (OverlappedComponent :type Primitive%20Component%20Object%20Reference) (OtherActor :type Actor%20Object%20Reference) (OtherComp :type Primitive%20Component%20Object%20Reference) (OtherBodyIndex :type Integer) (bFromSweep :type Boolean) (SweepResult :type Hit%20Result%20Structure%20%28by%20ref%29))
  (Utilities|Casting|CastToBP_Chicken OtherActor)
  (Actor|DestroyActor))

(event OnComponentHit(StaticMesh_0)
  (params (HitComponent :type Primitive%20Component%20Object%20Reference) (OtherActor :type Actor%20Object%20Reference) (OtherComp :type Primitive%20Component%20Object%20Reference) (NormalImpulse :type Vector :default "0, 0, 0") (Hit :type Hit%20Result%20Structure%20%28by%20ref%29))
  (Utilities|FlowControl|DoOnce false
    (:Completed
      (Utilities|Casting|CastToBP_Chicken OtherActor)
      (bind _ascrossy_gm (Utilities|Casting|CastToCrossy_GM (Game|GetGameMode)))
      (Variables|/Game/GameModes/Crossy_GM.Crossy_GM_C|SetScore _ascrossy_gm (+ 1 (Variables|/Game/GameModes/Crossy_GM.Crossy_GM_C|GetScore _ascrossy_gm))))))

(event EventBeginPlay
  (|CallParentFunction)
  (CallFunction|SpawnCoin))

(event Collision|EventActorBeginOverlap
  (params (OtherActor :type Actor%20Object%20Reference)))

(event EventTick
  (params (DeltaSeconds :type Float%20%28single-precision%29))
  (Utilities|FlowControl|Delay 1.5)
  (if (Math|Random|RandomBool)
    (CallFunction|SpawnCars)
    (else
      (CallFunction|SpawnTruck))))

(fn ConstructionScript
  (|CallParentFunction))

(fn SpawnCars
  (switch int (Math|Random|RandomIntegerinRange 0 1)
    (:1
      (Game|SpawnActorfromClass "/Game/Blueprints/BP_Cars.BP_Cars_C" (Transformation|GetWorldTransform (Variables|Default|GetSpawnCar)) "Undefined" 0 0))))

(fn SpawnTruck
  (switch int (Math|Random|RandomIntegerinRange 0 1)
    (:1
      (Game|SpawnActorfromClass "/Game/Blueprints/BP_Truck.BP_Truck_C" (Transformation|GetWorldTransform (Variables|Default|GetSpawnTrucks)) "Undefined" 0 0))))

(fn SpawnCoin
  (switch int (Math|Random|RandomIntegerinRange 0 5)
    (:0
      (Game|SpawnActorfromClass "/Game/Blueprints/BP_Coin.BP_Coin_C" (Transformation|GetWorldTransform (Variables|Default|GetArrow12)) "Undefined" 0 0)
      (switch int (Math|Random|RandomIntegerinRange 0 5)
        (:0
          (Game|SpawnActorfromClass "/Game/Blueprints/BP_Coin.BP_Coin_C" (Transformation|GetWorldTransform (Variables|Default|GetArrow13)) "Undefined" 0 0)
          (switch int (Math|Random|RandomIntegerinRange 0 5)
            (:0
              (Game|SpawnActorfromClass "/Game/Blueprints/BP_Coin.BP_Coin_C" (Transformation|GetWorldTransform (Variables|Default|GetArrow14)) "Undefined" 0 0))))))))